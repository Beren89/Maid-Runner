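; A sink actor that collects actors tagged "Pot" and signals when it has received two.
; When a tagged actor overlaps its Box, the sink destroys it and adds a scaled static mesh component in its place, offset along Y by the Bowl counter.
; The counter then increments, and reaching two calls the SinkDone event dispatcher.
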(event `self.Box.OnComponentBeginOverlap`
  (params (OtherActor :type "Actor Object Reference") (OtherComp :type "PrimitiveComponent Object Reference") (OtherBodyIndex :type Integer) (bFromSweep :type Boolean) (SweepResult :type "HitResult Structure (by ref)"))
  (if (`self.ActorHasTag` OtherActor "Pot")
    (`self.K2_DestroyActor` OtherActor)
    (`AddComponent|StaticMeshComponent_981` :`RelativeTransform` (`KismetMathLibrary.MakeTransform` (`KismetMathLibrary.MakeVector` -40.0 (* (`self.bowl`) 110.0) 200.0) (struct :`Yaw` 220.0) (0.6 0.6 0.6)))
    (bind _output_get (set `self.bowl` (+ (`self.bowl`) 1)))
    (if (== _output_get 2)
      (`self.SinkDone`))))

(fn `UserConstructionScript`)