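; FinnHUD is a HUD that shows story clues and next-objective hints, from a secret project conversation through a safe code to a win message.
; DrawHUD draws TextContent1 horizontally centered near the screen bottom.
; The Text1 event takes five booleans, and the first true one selects a two-message sequence timed by delays, then clears the text.
; Each branch also wires directly into the DrawText node.
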(event `self.ReceiveDrawHUD`
  (params (SizeX :type Integer) (SizeY :type Integer))
  (set `self.SizeX` SizeX)
  (set `self.SizeY` SizeY)
  (`self.DrawText` (`self.TextContent1`) (struct :`A` 1.0) (`KismetMathLibrary.Conv_IntToDouble` (/ (- (`self.SizeX`) (`KismetMathLibrary.FFloor` (`self.GetTextSize` (`self.TextContent1`) null 3.0))) 2)) (`KismetMathLibrary.Conv_IntToDouble` (- (`self.SizeY`) 50)) "/Engine/EngineFonts/Roboto.Roboto" 3.0 :!label _label))

(event `/Game/Blueprints/Gramophone_Interactions.Text1`
  (params (Text1 :type Boolean) (Text2 :type Boolean) (Text3 :type Boolean) (Text4 :type Boolean) (Text5 :type Boolean))
  (if Text1
    (`|ExecutionSequence`
      (:`then_0`
        (goto _label))
      (:`then_1`
        (set `self.TextContent1` "Conversation about secret project")
        (`KismetSystemLibrary.Delay` 2.0)
        (set `self.TextContent1` "Go look for books")
        (`KismetSystemLibrary.Delay` 2.0)
        (set `self.TextContent1` "" :!label _label_2)))
    (elif Text2
      (`|ExecutionSequence`
        (:`then_0`
          (goto _label))
        (:`then_1`
          (set `self.TextContent1` "Prototype discussions")
          (`KismetSystemLibrary.Delay` 2.0)
          (set `self.TextContent1` "Look for the prototype in the display case")
          (`KismetSystemLibrary.Delay` 2.0)
          (goto _label_2)))
      (elif Text3
        (`|ExecutionSequence`
          (:`then_0`
            (goto _label))
          (:`then_1`
            (set `self.TextContent1` "Writing of a contract")
            (`KismetSystemLibrary.Delay` 2.0)
            (set `self.TextContent1` "Go check near the drinks")
            (`KismetSystemLibrary.Delay` 2.0)
            (goto _label_2)))
        (elif Text4
          (`|ExecutionSequence`
            (:`then_0`
              (goto _label))
            (:`then_1`
              (set `self.TextContent1` "Contract")
              (`KismetSystemLibrary.Delay` 2.0)
              (set `self.TextContent1` "Key to the safe is 9573")
              (`KismetSystemLibrary.Delay` 2.0)
              (goto _label_2)))
          (elif Text5
            (`|ExecutionSequence`
              (:`then_0`
                (goto _label))
              (:`then_1`
                (set `self.TextContent1` "Life work, fluff and stuff")
                (`KismetSystemLibrary.Delay` 2.0)
                (set `self.TextContent1` "You won and shit")
                (`KismetSystemLibrary.Delay` 2.0)
                (goto _label_2)))))))))

(fn `Safe_Variable`
  (returns (Safe :type Integer))
  (return 0))

(fn `UserConstructionScript`)