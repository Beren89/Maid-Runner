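; Piano puzzle helper that releases music sheets as a movable object and detects when they are put in place.
; Interact reveals the sheets and plays a Matinee, then after a delay swaps them for a spawned MovableObj using the same mesh with overlap events enabled.
; When that object overlaps the Box, it is destroyed and SheetsInPlace is called.
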(event `/Game/Blueprints/Interact.Interact`
  (`SceneComponent.SetVisibility` (`self.Music Sheets`) true false)
  (`MatineeActor.Play` (`self.TargetMatinee`))
  (`KismetSystemLibrary.Delay` 2.0)
  (bind _returnvalue (`|SpawnActorFromClass` "/Game/Blueprints/MovableObj.MovableObj_C" (`SceneComponent.K2_GetComponentToWorld` (`self.Music Sheets`)) "Undefined" "OverrideRootScale"))
  (`SceneComponent.SetVisibility` (`self.Music Sheets`) false false)
  (bind _staticmeshcomponent (`StaticMeshActor.StaticMeshComponent` _returnvalue))
  (`StaticMeshComponent.SetStaticMesh` _staticmeshcomponent "/Game/Assets/MusicSheets_mesh.MusicSheets_mesh")
  (set `PrimitiveComponent.bGenerateOverlapEvents` true _staticmeshcomponent))

(event `self.Box.OnComponentBeginOverlap`
  (params (OtherActor :type "Actor Object Reference") (OtherComp :type "PrimitiveComponent Object Reference") (OtherBodyIndex :type Integer) (bFromSweep :type Boolean) (SweepResult :type "HitResult Structure (by ref)"))
  (if (== OtherActor (stale `/Game/Blueprints/Interact.Interact` _returnvalue))
    (`self.K2_DestroyActor` (stale `/Game/Blueprints/Interact.Interact` _returnvalue))
    (`self.Sheets in Place`)))

(fn `UserConstructionScript`)