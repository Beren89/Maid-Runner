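; Lazy waiter lift Blueprint that accepts platters delivered into its Box trigger and signals when the lift is done.
; An overlapping actor tagged "Platter" is destroyed and replaced by a scaled-down static mesh component attached at a fixed offset on the lift.
; A counter tracks received platters and fires CallLiftDone when the first one arrives.
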(event `self.Box.OnComponentBeginOverlap`
  (params (OtherActor :type "Actor Object Reference") (OtherComp :type "PrimitiveComponent Object Reference") (OtherBodyIndex :type Integer) (bFromSweep :type Boolean) (SweepResult :type "HitResult Structure (by ref)"))
  (if (`self.ActorHasTag` OtherActor "Platter")
    (`self.K2_DestroyActor` OtherActor)
    (`AddComponent|StaticMeshComponent_412` :`RelativeTransform` (`KismetMathLibrary.MakeTransform` (0.0 25.0 75.0) (struct) (0.2 0.2 0.2)))
    (bind _output_get (set `self.NewVar_0` (+ (`self.NewVar_0`) 1)))
    (if (== _output_get 1)
      (`self.LiftDone`))))

(fn `UserConstructionScript`)