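; Interactable lever that the player rotates with look input to activate a linked target.
; Interact sets RotationActive on the ThirdPersonCharacter and pitches LeverArm by the inverted look-up value.
; When LeverArm overlaps the trigger Box, it clears RotationActive, sends TriggerMessage to Target and calls TriggerActivated.
; BeginPlay applies the configurable arm and secondary meshes.
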(event `self.ReceiveBeginPlay`
  ;[1 1 1] Setting Lever and Secondary Meshes
  (`StaticMeshComponent.SetStaticMesh` (`self.ArmMesh`) (`self.Arm Mesh`))
  (`StaticMeshComponent.SetStaticMesh` (`self.SecondaryMesh`) (`self.Secondary Mesh`)))

(event `self.Box.OnComponentBeginOverlap`
  (params (OtherActor :type "Actor Object Reference") (OtherComp :type "PrimitiveComponent Object Reference") (OtherBodyIndex :type Integer) (bFromSweep :type Boolean) (SweepResult :type "HitResult Structure (by ref)"))
  ;[1 1 1] Activating Trigger Interface
  (if (== OtherComp (`self.Lever_arm`))
    (bind _asthird_person_character (cast `/Game/Blueprints/ThirdPersonCharacter` (`GameplayStatics.GetPlayerCharacter` 0)))
    (set `/Game/Blueprints/ThirdPersonCharacter.Rotation Active` false _asthird_person_character)
    (message `/Game/Blueprints/Triggers.Trigger` (`self.Target`))
    (`self.TriggerActivated`)))

(event `/Game/Blueprints/Interact.Interact`
  ;[1 1 1] Lever rotation
  (bind _asthird_person_character (cast `/Game/Blueprints/ThirdPersonCharacter` (`GameplayStatics.GetPlayerCharacter` 0)))
  (set `/Game/Blueprints/ThirdPersonCharacter.Rotation Active` true _asthird_person_character)
  (`SceneComponent.K2_AddLocalRotation` (`self.Lever_arm`) (`KismetMathLibrary.MakeRotator` 0.0 (* -1 (`self.GetInputAxisValue`))) false false))

(fn `UserConstructionScript`)